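; Attack component that gives its owning character a library of attacks: melee, ground smash, long-range leap slash, mage spell and projectile barrage.
; Montage attacks signal start and end to the owner through messages, with heavier moves disabling interruption.
; Montage notifies trigger sphere traces, spawned AOE actors, dark-energy projectiles or an arced launch toward the target.
; Trace and AOE damage skip same-team actors; a separate bullet helper damages the first non-teammate hit.
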(event `PrimaryMeleeAttack`
  (params (AttackInfo :type "/Game/Attacks/S_AttackInfo Structure") (`Sphere Trace Radius` :type "Float (double-precision)") (ActorFrowardLength :type "Float (double-precision)"))
  (bind (_attacktarget _attackmontage _damageinfo) (break `/Game/Attacks/S_AttackInfo` AttackInfo))
  ;[0.4678 0.4678 0.4678] Primary Melee Attack
  (bind _mesh (`self.AttackBase` _attacktarget))
  (bind _notifyname (`|PlayMontage` _mesh _attackmontage)
    (:`OnCompleted`
      (message `/Game/Enemy/BPI_Enemy.AttackEnd` (`self.GetOwner`) _attacktarget :!label _label))
    (:`OnInterrupted`
      (goto _label))
    (:`OnNotifyBegin`
      (switch `name` _notifyname
        (:`Slash`
          (`self.SphereTraceDamage` _damageinfo `Sphere Trace Radius` ActorFrowardLength))))))

(event `FireBullet`
  (params (TraceStart :type "Vector Structure") (TraceEnd :type "Vector Structure") (DamageInfo :type "/Game/DamageSystem/S_DamageInfo Structure"))
  ;[1 0.8755 0] Attack Helper
  (bind (_outhits _returnvalue) (`KismetSystemLibrary.LineTraceMultiForObjects` TraceStart TraceEnd (`|MakeArray` "ObjectTypeQuery3" :!type "EObjectTypeQuery Enum") false (`|MakeArray` (`self.GetOwner`)) "Persistent"))
  (if _returnvalue
    (bind _damagedatctor (`self.Damage First Non Team Members` _outhits DamageInfo))
    (`AISense_Damage.ReportDamageEvent` _damagedatctor (`self.GetOwner`) (`.Amount_2_64864A0D4320D27C3EA14D8019B5EC9D` (break `/Game/DamageSystem/S_DamageInfo` DamageInfo)) (`Actor.K2_GetActorLocation` (`self.GetOwner`)))))

(event `GroundSmash`
  (params (`Attack Info` :type "/Game/Attacks/S_AttackInfo Structure") (`AOE Radius` :type "Float (double-precision)"))
  (bind (_attacktarget _attackmontage _damageinfo) (break `/Game/Attacks/S_AttackInfo` `Attack Info`))
  (bind _returnvalue (`self.GetOwner`))
  ;[0.4678 0.4678 0.4678] Ground Smash
  (bind _mesh (`self.AttackBase` _attacktarget))
  (bind _notifyname (`|PlayMontage` _mesh _attackmontage)
    (:`then`
      (message `/Game/DamageSystem/BPI_Damagable.SetIsInterruptible` _returnvalue false))
    (:`OnCompleted`
      (message `/Game/Enemy/BPI_Enemy.AttackEnd` _returnvalue _attacktarget :!label _label_2)
      (message `/Game/DamageSystem/BPI_Damagable.SetIsInterruptible` _returnvalue true))
    (:`OnInterrupted`
      (goto _label_2))
    (:`OnNotifyBegin`
      (switch `name` _notifyname
        (:`Smash`
          (`self.AOEDamage` `AOE Radius` _damageinfo))))))

(event `MagicSpell`
  (params (SpawnTransform :type "Transform Structure") (Target :type "Actor Object Reference") (DamageInfo :type "/Game/DamageSystem/S_DamageInfo Structure"))
  ;[1 0.8755 0] Attack Helper
  (bind _returnvalue (`|SpawnActorFromClass` "/Game/Projectiles/BP_Projectile_DarkEnergy.BP_Projectile_DarkEnergy_C" SpawnTransform "Undefined" "MultiplyWithRoot" (`self.GetOwner`) 500.0 0.0 Target false null))
  (add `/Game/Projectiles/BP_Projectile_Base.OnProjectileImpact` _returnvalue (delegate `OnProjectileHit`))
  (`PrimitiveComponent.IgnoreActorWhenMoving` (`Actor.GetComponentByClass` (`self.GetOwner`) "/Script/Engine.CapsuleComponent") _returnvalue true))

(event `OnProjectileHit`
  (params (OtherActor :type "Actor Object Reference") (Hit :type "HitResult Structure"))
  ;[1 0.8755 0] Attack Helper
  (message `/Game/DamageSystem/BPI_Damagable.TakeDamage` OtherActor (stale `MagicSpell` DamageInfo) (`self.GetOwner`))
  (`AISense_Damage.ReportDamageEvent` OtherActor (`self.GetOwner`) (`.Amount_2_64864A0D4320D27C3EA14D8019B5EC9D` (break `/Game/DamageSystem/S_DamageInfo` (stale `MagicSpell` DamageInfo))) (`Actor.K2_GetActorLocation` (`self.GetOwner`)))
  (`self.OnAttackEnded`))

(event `LongRangeMeleeAttack`
  (params (`Attack Info` :type "/Game/Attacks/S_AttackInfo Structure"))
  (bind (_attacktarget _attackmontage _damageinfo) (break `/Game/Attacks/S_AttackInfo` `Attack Info`))
  (bind _returnvalue (`self.GetOwner`))
  ;[0 0.4678 0.4427] Long Range Melee Attack
  (bind _mesh (`self.AttackBase` _attacktarget))
  (bind _notifyname (`|PlayMontage` _mesh _attackmontage)
    (:`then`
      (message `/Game/DamageSystem/BPI_Damagable.SetIsInterruptible` _returnvalue false))
    (:`OnCompleted`
      (message `/Game/Enemy/BPI_Enemy.AttackEnd` _returnvalue _attacktarget :!label _label_3)
      (message `/Game/DamageSystem/BPI_Damagable.SetIsInterruptible` _returnvalue true))
    (:`OnInterrupted`
      (goto _label_3))
    (:`OnNotifyBegin`
      (switch `name` _notifyname
        (:`Slash`
          (`self.SphereTraceDamage` _damageinfo 20.0 200.0))
        (:`Jump`
          (`self.JumpToAttackTarget` _attacktarget))
        (:`AOESlash`
          (`self.AOEDamage` 0.0 _damageinfo))))))

(event `AOEDamage`
  (params (`AOE Radius` :type "Float (double-precision)") (DamageInfo :type "/Game/DamageSystem/S_DamageInfo Structure"))
  (bind _returnvalue (`self.GetOwner`))
  ;[1 0.8755 0] Attack Helper
  (bind _returnvalue_2 (`|SpawnActorFromClass` "/Game/AOE/BP_AOE_Base.BP_AOE_Base_C" (`KismetMathLibrary.MakeTransform` (`Actor.K2_GetActorLocation` _returnvalue)) "Undefined" "MultiplyWithRoot" null false true false (cast `Pawn` _returnvalue :!pure true)))
  (set `/Game/AOE/BP_AOE_Base.Radius` `AOE Radius` _returnvalue_2)
  (add `/Game/AOE/BP_AOE_Base.OnAOEOverlapActor` _returnvalue_2 (delegate `AOEDamageActor`))
  (`/Game/AOE/BP_AOE_Base.Trigger` _returnvalue_2))

(event `AOEDamageActor`
  (params (Actor :type "Actor Object Reference"))
  ;[1 0.8755 0] Attack Helper
  (bind _teamnumber (message `/Game/DamageSystem/BPI_Damagable.GetTeamNumber` Actor))
  (bind _teamnumber_2 (message `/Game/DamageSystem/BPI_Damagable.GetTeamNumber` (`self.GetOwner`)))
  (if (!= _teamnumber_2 _teamnumber)
    (message `/Game/DamageSystem/BPI_Damagable.TakeDamage` Actor (stale `AOEDamage` DamageInfo) (`self.GetOwner`))))

(event `SphereTraceDamage`
  (params (DamageInfo :type "/Game/DamageSystem/S_DamageInfo Structure") (`Sphere Radius` :type "Float (double-precision)") (`Actor Forward Length` :type "Float (double-precision)"))
  (bind _returnvalue (`self.GetOwner`))
  (bind _returnvalue_2 (`Actor.K2_GetActorLocation` _returnvalue))
  ;[1 0.8755 0] Attack Helper
  (bind (_outhits _returnvalue_3) (`KismetSystemLibrary.SphereTraceMultiForObjects` _returnvalue_2 (+ _returnvalue_2 (* (`Actor.GetActorForwardVector` _returnvalue) `Actor Forward Length`)) `Sphere Radius` (`|MakeArray` "ObjectTypeQuery3" :!type "EObjectTypeQuery Enum")))
  (if _returnvalue_3
    (`self.Damage All Non Team Members` _outhits DamageInfo)))

(event `BasicMageSpell`
  (params (AttackInfo :type "/Game/Attacks/S_AttackInfo Structure"))
  (bind (_attacktarget _attackmontage _damageinfo) (break `/Game/Attacks/S_AttackInfo` AttackInfo))
  ;[0.4678 0.4678 0.4678] Basic Mage Spell
  (bind _mesh (`self.AttackBase` _attacktarget))
  (bind _notifyname (`|PlayMontage` _mesh _attackmontage)
    (:`OnCompleted`
      (message `/Game/Enemy/BPI_Enemy.AttackEnd` (`self.GetOwner`) _attacktarget :!label _label_4))
    (:`OnInterrupted`
      (goto _label_4))
    (:`OnNotifyBegin`
      (switch `name` _notifyname
        (:`Fire`
          (`self.MagicSpell` (`KismetMathLibrary.MakeTransform` (`SceneComponent.GetSocketLocation` _mesh "RightHand")) _attacktarget _damageinfo))))))

(event `BarrageAttack`
  (params (AttackInfo :type "/Game/Attacks/S_AttackInfo Structure"))
  (bind (_attacktarget _attackmontage _damageinfo) (break `/Game/Attacks/S_AttackInfo` AttackInfo))
  (bind _returnvalue (`self.GetOwner`))
  ;[0.4678 0.4678 0.4678] BarrageAttack
  (bind _mesh (`self.AttackBase` _attacktarget))
  (bind _notifyname (`|PlayMontage` _mesh _attackmontage)
    (:`then`
      (message `/Game/DamageSystem/BPI_Damagable.SetIsInterruptible` _returnvalue false))
    (:`OnCompleted`
      (message `/Game/Enemy/BPI_Enemy.AttackEnd` _returnvalue _attacktarget :!label _label_5)
      (message `/Game/DamageSystem/BPI_Damagable.SetIsInterruptible` _returnvalue true))
    (:`OnInterrupted`
      (goto _label_5))
    (:`OnNotifyBegin`
      (switch `name` _notifyname
        (:`Fire`
          (`self.MagicSpell` (`KismetMathLibrary.MakeTransform` (`SceneComponent.GetSocketLocation` _mesh "RightHand") (`KismetMathLibrary.FindLookAtRotation` (`Actor.K2_GetActorLocation` (`self.GetOwner`)) (+ (`Actor.K2_GetActorLocation` _attacktarget) (`KismetMathLibrary.MakeVector` 0.0 (`KismetMathLibrary.RandomFloatInRange` -150.0 150.0))))) null _damageinfo))))))

(event `JumpToAttackTarget`
  (params (AttackTarget :type "Actor Object Reference"))
  (bind `_as角色` (cast `Character` (`self.GetOwner`) :!pure true))
  ;[1 0.8755 0] Attack Helper
  (bind _location (`self.CalculateFutureActorLocation` AttackTarget))
  (bind _outlaunchvelocity (`GameplayStatics.SuggestProjectileVelocity_CustomArc` (`Actor.K2_GetActorLocation` (`self.GetOwner`)) (`KismetMathLibrary.MakeVector` (.x _location) (.y _location) (+ (.z _location) 100.0)) 0.0 (`KismetMathLibrary.Lerp` 0.5 0.94 (`KismetMathLibrary.FClamp` (`KismetMathLibrary.NormalizeToRange` (`Actor.GetDistanceTo` AttackTarget (`self.GetOwner`)) 400.0 800.0)))))
  (`Character.LaunchCharacter` `_as角色` _outlaunchvelocity true true)
  (add `Character.LandedDelegate` `_as角色` (delegate `OnLand`)))

(event `OnLand`
  (params (Hit :type "HitResult Structure (by ref)"))
  (bind `_as角色` (cast `Character` (`self.GetOwner`) :!pure true))
  ;[1 0.8755 0] Attack Helper
  (remove `Character.LandedDelegate` `_as角色` (delegate `OnLand`))
  (`MovementComponent.StopMovementImmediately` (`Character.CharacterMovement` `_as角色`)))

(fn `AttackBase`
  (params (AttackTarget :type "Actor Object Reference"))
  (returns (Mesh :type "SkeletalMeshComponent Object Reference"))
  (bind _returnvalue (`self.GetOwner`))
  ; 调用 Attack 函数
  (message `/Game/Enemy/BPI_Enemy.Attack` _returnvalue AttackTarget)
  (bind `_as角色` (cast `Character` _returnvalue))
  (return (`Character.Mesh` `_as角色`)))

(fn `CalculateFutureActorLocation`
  (params (Actor :type "Actor Object Reference") (Time :type "Float (double-precision)"))
  (returns (Location :type "Vector Structure"))
  (return (+ (`Actor.K2_GetActorLocation` Actor) (* (* (`Actor.GetVelocity` Actor) (1.0 1.0 0.0)) Time))))

(fn `Damage All Non Team Members`
  (params (Hits :type "Array of HitResult Structure") (DamageInfo :type "/Game/DamageSystem/S_DamageInfo Structure"))
  (returns (ActorsDamage :type "Array of Actor Object Reference"))
  (locals (ActorsDamgedAlready :type "Array of Actor Object Reference"))
  (for _array_element Hits
    (bind (_bblockinghit _binitialoverlap _time _distance _location _impactpoint _normal _impactnormal _physmat _hitactor) (`GameplayStatics.BreakHitResult` _array_element))
    (bind _teamnumber (message `/Game/DamageSystem/BPI_Damagable.GetTeamNumber` _hitactor))
    (bind _teamnumber_2 (message `/Game/DamageSystem/BPI_Damagable.GetTeamNumber` (`self.GetOwner`)))
    (if (and (!= _teamnumber_2 _teamnumber) (not (`KismetArrayLibrary.Array_Contains` (`local.ActorsDamgedAlready`) _hitactor)))
      (message `/Game/DamageSystem/BPI_Damagable.TakeDamage` _hitactor DamageInfo (`self.GetOwner`))
      (`KismetArrayLibrary.Array_AddUnique` (`local.ActorsDamgedAlready`) _hitactor)))
  (return (`local.ActorsDamgedAlready`)))

(fn `Damage First Non Team Members`
  (params (Hits :type "Array of HitResult Structure") (DamageInfo :type "/Game/DamageSystem/S_DamageInfo Structure"))
  (returns (DamagedAtctor :type "Actor Object Reference"))
  (for _array_element Hits
    (bind (_bblockinghit _binitialoverlap _time _distance _location _impactpoint _normal _impactnormal _physmat _hitactor) (`GameplayStatics.BreakHitResult` _array_element))
    (bind _teamnumber (message `/Game/DamageSystem/BPI_Damagable.GetTeamNumber` _hitactor))
    (bind _teamnumber_2 (message `/Game/DamageSystem/BPI_Damagable.GetTeamNumber` (`self.GetOwner`)))
    (if (!= _teamnumber_2 _teamnumber)
      (message `/Game/DamageSystem/BPI_Damagable.TakeDamage` _hitactor DamageInfo (`self.GetOwner`))
      (`|ExecutionSequence`
        (:`then_0`
          (break))
        (:`then_1`
          (return _hitactor))))))