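; Boss enemy Blueprint that extends a parent enemy class, with 500 health and an axe as its weapon.
; The construction script sets max and current health on the damage system component.
; On BeginPlay it spawns the axe, snaps it to the mesh's AxeSocket, then signals equipped a tick later.
; Unequipping signals first, then destroys WeaponActor a tick later, a different variable from the spawned WeaponAxe.
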(event `self.ReceiveBeginPlay`
  (`parent.ReceiveBeginPlay`)
  (`/Game/Enemy/BPI_Enemy.EquipWeapon`))

(event `/Game/Enemy/BPI_Enemy.EquipWeapon`
  (bind _returnvalue (`|SpawnActorFromClass` "/Game/Weapons/BP/BP_Weapon_Axe.BP_Weapon_Axe_C" (`KismetMathLibrary.MakeTransform` (0.0 0.0 0.0)) "Undefined" "MultiplyWithRoot" null null))
  (bind _output_get (set `self.WeaponAxe` _returnvalue))
  (`self.K2_AttachToComponent` _output_get (`self.Mesh`) "AxeSocket" "SnapToTarget" "SnapToTarget" "SnapToTarget" true)
  (`KismetSystemLibrary.DelayUntilNextTick`)
  (`self.OnWeaponEquipped`)
  (set `self.bIsWieldingWeapon` true))

(event `/Game/Enemy/BPI_Enemy.UnequipWeapon`
  (`self.OnWeaponUnequipped`)
  (`KismetSystemLibrary.DelayUntilNextTick`)
  (`self.K2_DestroyActor` (`self.WeaponActor`))
  (set `self.bIsWieldingWeapon` false))

(fn `UserConstructionScript`
  (bind _bpc_damagesystem (`self.BPC_DamageSystem`))
  (`parent.UserConstructionScript`)
  (bind _output_get (set `/Game/DamageSystem/BPC_DamageSystem.MaxHealth` 500.0 _bpc_damagesystem))
  (set `/Game/DamageSystem/BPC_DamageSystem.Health` _output_get _bpc_damagesystem))