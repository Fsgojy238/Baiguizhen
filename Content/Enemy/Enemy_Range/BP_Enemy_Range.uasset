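; BP_Enemy_Range is the ranged rifle enemy, a child of a parent enemy Blueprint.
; On BeginPlay it spawns a rifle and attaches it to the mesh's RifleSocket.
; Attack plays a rifle-fire montage and calls AttackEnd on completion or interruption, but the FireBullet trace call is left disconnected.
; It also defines walk speeds per locomotion state and its ideal attack and strafe ranges.
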(event `self.ReceiveBeginPlay`
  (`parent.ReceiveBeginPlay`)
  (`self.EquipWeapon`))

(event `/Game/Enemy/BPI_Enemy.EquipWeapon`
  (bind _returnvalue (`|SpawnActorFromClass` "/Game/Weapons/BP/BP_Weapon_Rifle.BP_Weapon_Rifle_C" (`self.GetTransform`) "Undefined" "MultiplyWithRoot" null null))
  (bind _output_get (set `self.WeaponActor` _returnvalue))
  (`self.K2_AttachToComponent` _output_get (`self.Mesh`) "RifleSocket" "SnapToTarget" "SnapToTarget" "SnapToTarget" true)
  (set `self.bIsWieldingWeapon` true))

(event `/Game/Enemy/BPI_Enemy.Attack`
  (params (AttackTarget :type "Actor Object Reference"))
  (`parent.Attack` AttackTarget)
  (bind _notifyname (`|PlayMontage` (`self.Mesh`) "/Game/Enemy/Enemy_Range/Anim/Montages/rifle-fire_Montage.rifle-fire_Montage")
    (:`OnCompleted`
      (`self.AttackEnd` AttackTarget :!label _label))
    (:`OnInterrupted`
      (goto _label))
    (:`OnNotifyBegin`
      (switch `name` _notifyname))))

(fn `GetIdealRange`
  (returns (AttackRadius :type "Float (double-precision)") (StrafeRadius :type "Float (double-precision)"))
  (return 600.0 600.0))

(fn `SetMovementSpeed`
  (params (InLocomotionState :type "/Game/Enemy/AI/Enum/E_LocomotionState Enum" :default "NewEnumerator0"))
  (returns (Speed :type "Float (double-precision)"))
  (bind _output_get (set `CharacterMovementComponent.MaxWalkSpeed` (select `/Game/Enemy/AI/Enum/E_LocomotionState` InLocomotionState :`NewEnumerator1` 150.0 :`NewEnumerator2` 200.0 :`NewEnumerator3` 500.0 :`NewEnumerator5` 300.0 :!type "Float (single-precision)") (`self.CharacterMovement`)))
  (return _output_get))

(fn `UserConstructionScript`
  (`parent.UserConstructionScript`))