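; Player action character Blueprint with sword and gun stances, built on an ability system.
; Aim input toggles between movement-oriented and controller-facing rotation, switches the skill link tag between Sword and Gun, resets input state and pushes a camera mode.
; BeginPlay feeds the body and sword meshes to the attack collision component.
; A dash flag triggers a one-shot snap to input direction, and being attacked applies a test hurt GameplayEffect to itself.
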(event `self.ReceiveBeginPlay`
  (`AttackCollisionComponent.SetSkeletalMeshAndStaticMesh` (`self.AttackCollisionComponent`) (`self.Mesh`) (`self.Sword`)))

(event `GlobalAttributeInterface.OnAttributeChanged`
  (params (AttributeData :type "GameplayAttributeData Structure (by ref)"))
  (`KismetSystemLibrary.PrintString` (`KismetStringLibrary.Conv_DoubleToString` AttributeData_CurrentValue)))

(event `self.ReceiveTick`
  (params (DeltaSeconds :type "Float (single-precision)"))
  (`parent.ReceiveTick` DeltaSeconds)
  (if (`self.bDashRotation`)
    (`self.UpdatePlayerRotation`)))

(event `EnhancedInput|/Game/Input/NormalInput/Aim`
  (params (ActionValue :type "Vector2D Structure") (ElapsedSeconds :type "Float (double-precision)") (TriggeredSeconds :type "Float (double-precision)") (InputAction :type "InputAction Object Reference" :default "/Game/Input/NormalInput/Aim.Aim"))
  (bind _actionabilitysystemcomponent (`self.ActionAbilitySystemComponent`))
  (bind _playercameramanager (`PlayerController.PlayerCameraManager` (`self.GetLocalViewingPlayerController`)))
  (:`Started`
    (`self.ChangeMovementType` false)
    (`SkillManager.ChangeSkillAssetLinkTag` (`ActionAbilitySystemComponent.GetSkillManager` (`self.ActionAbilitySystemComponent`)) (struct :`TagName` "WeaponTag.Gun"))
    (`ActionAbilitySystemComponent.SetCurrentInputState` _actionabilitysystemcomponent "NormalInputState")
    (bind _asbp_action_camera_manager (cast `/Game/Gameplay/CameraSystem/BP_ActionCameraManager` _playercameramanager))
    (`ActionPlayerCameraManager.PushCameraMode` _asbp_action_camera_manager "/Game/Gameplay/CameraSystem/CameraMode/AimCameraMode.AimCameraMode_C"))
  (:`Completed`
    (`self.ChangeMovementType` true)
    (`SkillManager.ChangeSkillAssetLinkTag` (`ActionAbilitySystemComponent.GetSkillManager` _actionabilitysystemcomponent) (struct :`TagName` "WeaponTag.Sword"))
    (`ActionAbilitySystemComponent.SetCurrentInputState` _actionabilitysystemcomponent "NormalInputState")
    (bind _asbp_action_camera_manager_2 (cast `/Game/Gameplay/CameraSystem/BP_ActionCameraManager` _playercameramanager))
    (`ActionPlayerCameraManager.PushCameraMode` _asbp_action_camera_manager_2 "/Game/Gameplay/CameraSystem/CameraMode/TestCameraMode.TestCameraMode_C")))

(event `CollisionSystemInterface.OnBeAttackRecallInternal`
  (params (AttackedResult :type "AttackedResult Structure"))
  (`AbilitySystemComponent.BP_ApplyGameplayEffectToTarget` :`self` (`self.ActionAbilitySystemComponent`) :`GameplayEffectClass` "/Game/Character/GE_HurtTest.GE_HurtTest_C" :`Target` (`self.ActionAbilitySystemComponent`)))

(fn `ChangeMovementType`
  (params (bPivotMovement :type Boolean))
  (bind _charactermovement (`self.CharacterMovement`))
  (bind _charactermovement_2 (`self.CharacterMovement`))
  (if bPivotMovement
    (set `CharacterMovementComponent.bUseControllerDesiredRotation` false _charactermovement)
    (set `CharacterMovementComponent.bOrientRotationToMovement` true _charactermovement)
    (set `self.AimCamera` false)
    (else
      (set `CharacterMovementComponent.bUseControllerDesiredRotation` true _charactermovement_2)
      (set `CharacterMovementComponent.bOrientRotationToMovement` false _charactermovement_2)
      (set `self.AimCamera` true))))

(fn `GetAttackCollisionComponent`
  (returns (ReturnValue :type "AttackCollisionComponent Object Reference"))
  (return (`self.AttackCollisionComponent`)))

(fn `UpdatePlayerRotation`
  (bind _returnvalue (`self.GetNormalInputData`))
  (bind _returnvalue_2 (`self.GetControlRotation`))
  (`self.K2_SetActorRotation` (`KismetMathLibrary.MakeRotFromX` (+ (* (`KismetMathLibrary.BreakVector2D` (break `CharacterNormalInputData` _returnvalue)) (`KismetMathLibrary.GetForwardVector` _returnvalue_2)) (* (`.Y` (`KismetMathLibrary.BreakVector2D` (break `CharacterNormalInputData` _returnvalue))) (`KismetMathLibrary.GetRightVector` _returnvalue_2)))) true)
  (set `self.bDashRotation` false))

(fn `UserConstructionScript`)